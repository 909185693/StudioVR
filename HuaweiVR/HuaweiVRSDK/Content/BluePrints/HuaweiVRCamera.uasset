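; Huawei VR camera Blueprint that shows headset system notifications in a floating message box in front of the player.
; Tick polls SDK messages, then controller plugin messages, spawning or reusing a message actor placed ahead of VRCamera and facing it.
; DynamicChangeUI sets icon, text and layout per message type.
; Messages auto-hide, except thermal warnings, which block other messages until dismissed by touch; an AppQuit warning triggers delayed quit.
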(event `self.ReceiveBeginPlay`
  ;[1 1 1] Enable helmet position and posture tracking
  (`HeadMountedDisplayFunctionLibrary.SetTrackingOrigin` "Eye")
  (`PlayerController.ActivateTouchInterface` (`GameplayStatics.GetPlayerController` 0) null))

(event `Key|Touch1`
  (params (Key :type "Key Structure"))
  (bind _huaweivrmessageactor (`self.HuaweiVRMessageActor`))
  ;[1 1 1] When you touch the touchpad or touch screen, the thermal message box will disappear
  (:`Released`
    (if (`self.ThermalMessageIsVisible`) :!label _label
      (`/Engine/EditorBlueprintResources/StandardMacros.IsValid` _huaweivrmessageactor
        (:`Is Valid`
          (`SceneComponent.SetVisibility` (`/HuaweiVRSDK/BluePrints/HuaweiVRMessageActor.Widget` _huaweivrmessageactor) false false)
          (set `self.ThermalMessageIsVisible` false))))))

(event `Key|MotionController_Right_FaceButton6`
  (params (Key :type "Key Structure"))
  ;[1 1 1] When you touch the touchpad or touch screen, the thermal message box will disappear
  (:`Released`
    (goto _label)))

(event `self.ReceiveTick`
  (params (DeltaSeconds :type "Float (single-precision)"))
  (bind _returnvalue_roll (`KismetMathLibrary.BreakRotator` (`self.K2_GetActorRotation`)))
  (bind _vrcamera (`self.VRCamera`))
  (bind _returnvalue (`SceneComponent.K2_GetComponentLocation` _vrcamera))
  (bind (_returnvalue_roll_2 _returnvalue_pitch _returnvalue_yaw) (`KismetMathLibrary.BreakRotator` (`SceneComponent.K2_GetComponentRotation` _vrcamera)))
  (bind _returnvalue_2 (`KismetMathLibrary.MakeRotator` 0.0 _returnvalue_pitch _returnvalue_yaw))
  (bind _returnvalue_3 (+ _returnvalue (* (`KismetMathLibrary.GetForwardVector` _returnvalue_2) (`self.DisplayForwardDistance`)) (* (`KismetMathLibrary.GetUpVector` _returnvalue_2) (`self.DisplayUpDistance`))))
  (bind (_returnvalue_roll_3 _returnvalue_pitch_2 _returnvalue_yaw_2) (`KismetMathLibrary.BreakRotator` (`KismetMathLibrary.FindLookAtRotation` _returnvalue_3 _returnvalue)))
  (bind (_type _priority _boxtype _message _returnvalue_4) (`HuaweiVRSDKBPFunctionLibrary.GetHuaweiVRMessage`))
  (bind _output_get (set `self.HasSDKMessage` _returnvalue_4))
  (if _output_get
    ;[1 1 1] Parse HuaweiVR Message
    (bind _output_get_2 (set `self.CurrentMessageType` _type))
    (if (`self.ThermalMessageIsVisible`)
      (if (`|EnumEquality` _output_get_2 "HuaweiVRMessage_ThermalWarning")
        (bind _output_get_3 (set `self.MessageMap` _message :!label _label_2))
        (set `self.CurrentMessagePriority` _priority)
        (bind (_value _returnvalue_5) (`BlueprintMapLibrary.Map_Find` _output_get_3 (`self.MessageKeyTitle`)))
        (if _returnvalue_5 :!label _label_3
          (set `self.HuaweiVRMessageTitle` _value))
        (bind (_value_2 _returnvalue_6) (`BlueprintMapLibrary.Map_Find` _output_get_3 (`self.MessageKeyContent`)))
        (if _returnvalue_6
          (set `self.HuaweiVRMessageContent` _value_2))
        (bind (_value_3 _returnvalue_7) (`BlueprintMapLibrary.Map_Find` _output_get_3 (`self.MessageKeyTips`)))
        (if _returnvalue_7
          (set `self.HuaweiVRMessageTips` _value_3))
        (bind (_value_4 _returnvalue_8) (`BlueprintMapLibrary.Map_Find` _output_get_3 (`self.MessageKeyExtention`)))
        (if _returnvalue_8
          (set `self.HuaweiVRMessageExtention` _value_4))
        ;[1 1 1] Create HuaweiVRMessageBox Dynamic
        (`/Engine/EditorBlueprintResources/StandardMacros.IsValid` (`self.HuaweiVRMessageActor`)
          (:`Is Valid`
            _)
          (:`Is Not Valid`
            (bind _returnvalue_9 (`|SpawnActorFromClass` (`self.HuaweiVRMessageActorClass`) (`KismetMathLibrary.MakeTransform` (0.0 0.0 0.0) (struct) (0.01 0.01 0.01)) "Undefined" "OverrideRootScale" null null))
            (bind _ashuawei_vrmessage_actor (cast `/HuaweiVRSDK/BluePrints/HuaweiVRMessageActor` _returnvalue_9))
            (bind _output_get_4 (set `self.HuaweiVRMessageActor` _ashuawei_vrmessage_actor))))
        (`self.DynamicChangeUI`)
        ;[1 1 1] Set message box location and rotation, and display it
        (`self.K2_SetActorLocation` _output_get_4 _returnvalue_3 false false)
        (`self.K2_SetActorRotation` _output_get_4 (`KismetMathLibrary.MakeRotator` _returnvalue_roll _returnvalue_pitch_2 _returnvalue_yaw_2) false)
        (`SceneComponent.SetVisibility` (`/HuaweiVRSDK/BluePrints/HuaweiVRMessageActor.Widget` (`self.HuaweiVRMessageActor`)) true false)
        (set `self.MessageBoxAppearTime` (`GameplayStatics.GetRealTimeSeconds`)))
      (else
        (goto _label_2)))
    (elif (not (`self.ThermalMessageIsVisible`))
      ;[1 1 1] Get message from controller plugin
      (bind (_type_2 _priority_2 _message_2 _returnvalue_10) (`HVRControllerFunctionLibrary.GetHVRControllerMessage`))
      (bind _output_get_5 (set `self.HasControllerMessage` _returnvalue_10))
      (if _output_get_5
        (set `self.MessageMap` _message_2)
        (set `self.ControllerMessageType` _type_2)
        (set `self.CurrentMessagePriority` _priority_2)
        (goto _label_3)
        (else
          ;[1 1 1] When HuaweiVR MessageBox shows more than ShowTime, it will be automatically detached
          (`/Engine/EditorBlueprintResources/StandardMacros.IsValid` (`self.HuaweiVRMessageActor`)
            (:`Is Valid`
              (if (> (- (`GameplayStatics.GetRealTimeSeconds`) (`self.MessageBoxAppearTime`)) (`self.MessageBoxShowTime`))
                (`SceneComponent.SetVisibility` (`/HuaweiVRSDK/BluePrints/HuaweiVRMessageActor.Widget` (`self.HuaweiVRMessageActor`)) false false)))))))))

(event `ThermalWarning_Level_3`
  (`KismetSystemLibrary.K2_SetTimer` null "AppQuitCountDown" 10.0))

(fn `AppQuitCountDown`
  (`KismetSystemLibrary.QuitGame` null "Quit"))

(fn `DynamicChangeUI`
  (bind _messageuiimagebox (`self.MessageUIImageBox`))
  (bind _messageuititle (`self.MessageUITitle`))
  (bind _messageuicontent (`self.MessageUIContent`))
  (bind _messageuitips (`self.MessageUITips`))
  (bind _messageuiicon (`self.MessageUIIcon`))
  (bind _messageuiicon_2 (`self.MessageUIIcon`))
  (bind _huaweivrmessageextention (`self.HuaweiVRMessageExtention`))
  (bind _messageuiicon_3 (`self.MessageUIIcon`))
  (bind _messageuiicon_4 (`self.MessageUIIcon`))
  (bind _messageuiicon_5 (`self.MessageUIIcon`))
  (bind _messageuiicon_6 (`self.MessageUIIcon`))
  (bind _returnvalue (`KismetStringLibrary.EqualEqual_StrStr` (`self.HuaweiVRMessageExtention`) "\"0\""))
  ;[1 1 1] Change the user interface dynamically
  (bind _ashuawei_vrmessage_box (cast `/HuaweiVRSDK/BluePrints/HuaweiVRMessageBox` (`WidgetComponent.GetUserWidgetObject` (`self.GetComponentByClass` (`self.HuaweiVRMessageActor`) "/Script/UMG.WidgetComponent")))
    (:`then`
      (set `self.MessageUIImageBox` (`/HuaweiVRSDK/BluePrints/HuaweiVRMessageBox.VerticalBox_Image` _ashuawei_vrmessage_box))
      (set `self.MessageUIIcon` (`/HuaweiVRSDK/BluePrints/HuaweiVRMessageBox.Image_MessageIcon` _ashuawei_vrmessage_box))
      (set `self.MessageUITips` (`/HuaweiVRSDK/BluePrints/HuaweiVRMessageBox.MultiLineEditableText_Tips` _ashuawei_vrmessage_box))
      (set `self.MessageUIContent` (`/HuaweiVRSDK/BluePrints/HuaweiVRMessageBox.MultiLineEditableText_Content` _ashuawei_vrmessage_box))
      (set `self.MessageUITitle` (`/HuaweiVRSDK/BluePrints/HuaweiVRMessageBox.MultiLineEditableText_Title` _ashuawei_vrmessage_box))
      (if (`self.HasSDKMessage`)
        (switch `HuaweiVRMessageType` (`self.CurrentMessageType`)
          (:`HuaweiVRMessage_NetWorkState`
            (if (`KismetStringLibrary.EqualEqual_StrStr` (`self.HuaweiVRMessageExtention`) "connected")
              (`Image.SetBrushFromTexture` _messageuiicon "/HuaweiVRSDK/Images/wificonnect.wificonnect" true)
              (else
                (`Image.SetBrushFromTexture` _messageuiicon "/HuaweiVRSDK/Images/wifidisconnect.wifidisconnect" true)))
            (`Widget.SetVisibility` _messageuiimagebox "Visible" :!label _label)
            (`Widget.SetVisibility` _messageuititle "Visible")
            (`Widget.SetVisibility` _messageuicontent "Collapsed")
            (`Widget.SetVisibility` _messageuitips "Collapsed")
            (`MultiLineEditableText.SetText` (`self.MessageUITitle`) (`KismetTextLibrary.Conv_StringToText` (`self.HuaweiVRMessageTitle`))))
          (:`HuaweiVRMessage_ThermalWarning`
            (set `self.ThermalMessageIsVisible` true)
            (if (`KismetStringLibrary.EqualEqual_StrStr` (`self.HuaweiVRMessageExtention`) "AppQuit")
              (`self.ThermalWarning_Level_3`))
            (`Widget.SetVisibility` _messageuiimagebox "Collapsed")
            (`Widget.SetVisibility` _messageuititle "Collapsed")
            (`Widget.SetVisibility` _messageuicontent "Visible")
            (`Widget.SetVisibility` _messageuitips "Visible")
            (`MultiLineEditableText.SetText` (`self.MessageUIContent`) (`KismetTextLibrary.Conv_StringToText` (`self.HuaweiVRMessageContent`)))
            (`MultiLineEditableText.SetText` (`self.MessageUITips`) (`KismetTextLibrary.Conv_StringToText` (`self.HuaweiVRMessageTips`))))
          (:`HuaweiVRMessage_NewSMS`
            (`Image.SetBrushFromTexture` _messageuiicon_2 "/HuaweiVRSDK/Images/message.message" true)
            (`Widget.SetVisibility` _messageuiimagebox "Visible" :!label _label_2)
            (`Widget.SetVisibility` _messageuititle "Visible")
            (`Widget.SetVisibility` _messageuicontent "Visible")
            (`Widget.SetVisibility` _messageuitips "Collapsed")
            (`MultiLineEditableText.SetText` (`self.MessageUITitle`) (`KismetTextLibrary.Conv_StringToText` (`self.HuaweiVRMessageTitle`)))
            (`MultiLineEditableText.SetText` (`self.MessageUIContent`) (`KismetTextLibrary.Conv_StringToText` (`self.HuaweiVRMessageContent`))))
          (:`HuaweiVRMessage_PhoneLowPower`
            (if _returnvalue
              (`Image.SetBrushFromTexture` _messageuiicon_2 "/HuaweiVRSDK/Images/phonelowpower_0.phonelowpower_0" true)
              (goto _label)
              (else
                (`Image.SetBrushFromTexture` _messageuiicon_2 "/HuaweiVRSDK/Images/phonelowpower_1.phonelowpower_1" true)
                (goto _label))))
          (:`HuaweiVRMessage_HelmetLowPower`
            (if _returnvalue
              (`Image.SetBrushFromTexture` _messageuiicon_3 "/HuaweiVRSDK/Images/helmetlowpower_0.helmetlowpower_0" true)
              (goto _label)
              (else
                (`Image.SetBrushFromTexture` _messageuiicon_3 "/HuaweiVRSDK/Images/helmetlowpower_1.helmetlowpower_1" true)
                (goto _label))))
          (:`HuaweiVRMessage_Common`
            (if (`KismetStringLibrary.EqualEqual_StrStr` (`self.WechatPackageName`) _huaweivrmessageextention)
              (`Image.SetBrushFromTexture` _messageuiicon_4 "/HuaweiVRSDK/Images/wechat.wechat" true)
              (goto _label_2)
              (elif (`KismetStringLibrary.EqualEqual_StrStr` _huaweivrmessageextention (`self.DeskClockPackageName`))
                (`Image.SetBrushFromTexture` _messageuiicon_4 "/HuaweiVRSDK/Images/alarm.alarm" true)
                (goto _label)))))
        (elif (`self.HasControllerMessage`)
          (switch `HVRControllerMessageType` (`self.ControllerMessageType`)
            (:`HVRControllerMessage_CaptureImageSucceed`
              _)
            (:`HVRControllerMessage_NoControllerJoin`
              (`Image.SetBrushFromTexture` _messageuiicon_6 "/HuaweiVRSDK/Images/controller_disconnected.controller_disconnected" true)
              (goto _label_2))
            (:`HVRControllerMessage_ControllerDisconnect`
              (`Image.SetBrushFromTexture` _messageuiicon_6 "/HuaweiVRSDK/Images/controller_disconnected.controller_disconnected" true)
              (goto _label))
            (:`HVRControllerMessage_CaptureImageFailed`
              _)
            (:`HVRControllerMessage_BluetoothDisable`
              (`Image.SetBrushFromTexture` _messageuiicon_5 "/HuaweiVRSDK/Images/bluetooth_disable.bluetooth_disable" true)
              (goto _label_2))
            (:`HVRControllerMessage_ControllerConnected`
              (`Image.SetBrushFromTexture` _messageuiicon_6 "/HuaweiVRSDK/Images/controller_connected.controller_connected" true)
              (goto _label)))
          (`Image.SetBrushFromTexture` _messageuiicon_5 "/HuaweiVRSDK/Images/screenshot.screenshot" true)
          (goto _label))))
    (:`CastFailed`
      (`KismetSystemLibrary.PrintString` "CastFailed" false))))

(fn `IsMessageAttached`
  (returns (Attatched :type Boolean))
  (bind _huaweivrmessageactor (`self.HuaweiVRMessageActor`))
  (`/Engine/EditorBlueprintResources/StandardMacros.IsValid` _huaweivrmessageactor
    (:`Is Valid`
      (return (== (`SceneComponent.GetAttachParent` (`/HuaweiVRSDK/BluePrints/HuaweiVRMessageActor.Widget` _huaweivrmessageactor)) (`self.VRCamera`))))
    (:`Is Not Valid`
      (return false))))

(fn `UserConstructionScript`)